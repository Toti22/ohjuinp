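; Player pawn Blueprint that handles movement, look, camera zoom and switching between the in-game interface and a map screen.
; Axis inputs drive forward and sideways movement and controller rotation, while Zoom and DeZoom presses set fixed camera FOVs.
; AfficheInterface shows the HUD on BeginPlay and map close, restoring game-only input.
; The Map action uses CanOpenMap and an InterfaceActuel string to toggle the map, pausing the game and showing the cursor.
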(event `InputAxis|Avancer/Reculer`
  (params (AxisValue :type "Float (single-precision)"))
  (`self.AddMovementInput` (`self.GetActorForwardVector`) AxisValue))

(event `InputAxis|VueVertical`
  (params (AxisValue :type "Float (single-precision)"))
  (`self.AddControllerPitchInput` AxisValue))

(event `InputAction|Zoom`
  (params (Key :type "Key Structure"))
  (:`Pressed`
    (`CameraComponent.SetFieldOfView` (`self.Camera`) 45.0)))

(event `InputAction|DeZoom`
  (params (Key :type "Key Structure"))
  (:`Pressed`
    (`CameraComponent.SetFieldOfView` (`self.Camera`) 90.0)))

(event `InputAxis|Tourner`
  (params (AxisValue :type "Float (single-precision)"))
  (`self.AddMovementInput` (`self.GetActorRightVector`) AxisValue))

(event `InputAxis|VueHorizontale`
  (params (AxisValue :type "Float (single-precision)"))
  (`self.AddControllerYawInput` AxisValue))

(event `AfficheInterface`
  (bind _returnvalue (`GameplayStatics.GetPlayerController` 0))
  (`WidgetLayoutLibrary.RemoveAllWidgets`)
  (bind _returnvalue_2 (`|CreateWidget` "/Game/HUD/Interface.Interface_C"))
  (`UserWidget.AddToViewport` _returnvalue_2 0)
  (`WidgetBlueprintLibrary.SetInputMode_GameOnly` _returnvalue)
  (set `PlayerController.bShowMouseCursor` false _returnvalue)
  (set `self.InterfaceActuel` "Interface"))

(event `InputAction|Map` :paused true
  (params (Key :type "Key Structure"))
  (bind _returnvalue (`GameplayStatics.GetPlayerController` 0))
  (:`Pressed`
    (if (`self.CanOpenMap`)
      (`WidgetLayoutLibrary.RemoveAllWidgets`)
      (bind _returnvalue_2 (`|CreateWidget` "/Game/HUD/Map.Map_C"))
      (`UserWidget.AddToViewport` _returnvalue_2 0)
      (`WidgetBlueprintLibrary.SetInputMode_GameAndUIEx` _returnvalue _returnvalue_2)
      (set `PlayerController.bShowMouseCursor` true _returnvalue)
      (set `self.CanOpenMap` false)
      (`GameplayStatics.SetGamePaused` true)
      (set `self.InterfaceActuel` "Map")
      (elif (`KismetStringLibrary.EqualEqual_StrStr` (`self.InterfaceActuel`) "Map")
        (set `self.CanOpenMap` true)
        (`self.AfficheInterface`)
        (`GameplayStatics.SetGamePaused` false)))))

(event `self.ReceiveBeginPlay`
  (`self.AfficheInterface`))

(fn `UserConstructionScript`)